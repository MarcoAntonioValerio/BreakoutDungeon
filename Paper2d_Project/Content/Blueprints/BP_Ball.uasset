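; BP_Ball is a physics-driven flipbook ball that the player holds and launches.
; While held, Tick snaps it to the player's hand position; LaunchBall sets its velocity, then after a short delay starts the trail and switches idle or spinning flipbook.
; Hits keep X velocity but randomize Z speed by its sign to control bounces, and overlapping the player turns the trail off after a delay.
; The animation switch re-applies the cached velocity because changing flipbooks kills it.
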(event OnComponentHit(Ball_Flipbook)
  (params (HitComponent :type Primitive%20Component%20Object%20Reference) (OtherActor :type Actor%20Object%20Reference) (OtherComp :type Primitive%20Component%20Object%20Reference) (NormalImpulse :type Vector :default "0, 0, 0") (Hit :type Hit%20Result%20Structure%20%28by%20ref%29))
  ;[1 1 1] Triggers on Hit.
  (CallFunction|ControlledBounce))

(event OnComponentBeginOverlap(Ball_Flipbook)
  (params (OverlappedComponent :type Primitive%20Component%20Object%20Reference) (OtherActor :type Actor%20Object%20Reference) (OtherComp :type Primitive%20Component%20Object%20Reference) (OtherBodyIndex :type Integer) (bFromSweep :type Boolean) (SweepResult :type Hit%20Result%20Structure%20%28by%20ref%29))
  ;[1 1 1] Activates the change flipbook event  when it starts to overlap.
  (Utilities|Casting|CastToBP_Player OtherActor)
  (Utilities|FlowControl|Delay 0.3)
  (CallFunction|DeactivateParticles))

(event Custom|LaunchBall
  ;[0.375 0.6159 1] Ball Launch        ➡️ ⚽
  ;;[1 1 1] Resets the linear velicity (to solve launch bug)
  (Physics|SetPhysicsLinearVelocity (Variables|Default|GetBall_Flipbook) "0, 0, 0" false "None")
  ;;[1 1 1] Adds the launching velocity to the ball!
  (Physics|SetPhysicsLinearVelocity (Variables|Default|GetBall_Flipbook) (Math|Vector|MakeVector (Variables|ExposedVariables|GetBall%20Velocity%20Value) 0.0 0.0) false "None")
  (Utilities|FlowControl|Delay 0.1)
  (CallFunction|ActivatesParticles)
  (CallFunction|FNCT|AnimationController))

(event Custom|Activates%20Particles
  ;[1 1 1] Particle Activator and Deactivator
  (Components|Activation|Activate (Variables|Default|GetTrail) false))

(event Custom|BallPositionBeforeLaunch
  (bind _player_actor_reference (Variables|References|GetPlayer%20Actor_Reference))
  ;[1 0.4989 0.6718] Hold Ball in "hands" before launch.                   ✋⚽🤚
  (if (Variables|/Game/Blueprints/BP_Player.BP_Player_C|GetAmIHoldingTheBall _player_actor_reference)
    ;;[1 1 1] Keeps the ball glued to the Player
    (Transformation|SetActorLocation (Variables|/Game/Blueprints/BP_Player.BP_Player_C|GetUpdatedHandPositionForBallCatch_0 _player_actor_reference) false false)))

(event Custom|Deactivate%20Particles
  ;[1 1 1] Particle Activator and Deactivator
  (Components|Activation|Deactivate (Variables|Default|GetTrail)))

(event Custom|Controlled%20Bounce
  ;[0.3083 0.3895 1] Bounce Controls
  ;;[1 1 1] Gets the velocity of the ball.
  (bind _returnvalue (Physics|GetPhysicsLinearVelocity (Variables|Default|GetBall_Flipbook) "None"))
  ;;[1 1 1] Sets the new velocity.
  (Physics|SetPhysicsLinearVelocity (Variables|Default|GetBall_Flipbook) (Math|Vector|MakeVector (.x _returnvalue) 0.0 (select (> (.z _returnvalue) 0.0) (Math|Random|RandomFloatinRange 4.5e+02 3e+02) (Math|Random|RandomFloatinRange -4.5e+02 -3e+02))) false "None"))

(event EventBeginPlay
  ;[0.3953 1 0.5746] Event Begin Play
  ;[1 1 1] Stores a connection to the player actor.
  (bind _returnvalue (Actor|GetActorOfClass "/Game/Blueprints/BP_Player.BP_Player_C"))
  (Variables|References|SetPlayer%20Actor_Reference _returnvalue))

(event EventTick
  (params (DeltaSeconds :type Float%20%28single-precision%29))
  ;[0.3385 0.1265 0.14] Event Tick
  (CallFunction|BallPositionBeforeLaunch)
  ;[1 1 1] Stores the X velocity for debug purposes.
  (bind _returnvalue (Physics|GetPhysicsLinearVelocity (Variables|Default|GetBall_Flipbook) "None"))
  (Variables|ExposedVariables|SetBallXVelocity (.x _returnvalue)))

(fn ConstructionScript)

(fn FNCT|AnimationController
  ;[1 1 1] Gets the velocity since we need it for multiple operations.
  (bind _returnvalue (Physics|GetPhysicsLinearVelocity (Variables|Default|GetBall_Flipbook) "None"))
  ;[1 1 1] Stores the current velocity for later.
  (bind _output_get (Variables|Default|SetCurrent%20Velocity _returnvalue))
  (Development|PrintString (Utilities|String|ToString(Vector) _output_get))
  ;[1 1 1] Check if velocity is not zero.
  (if (Class|KismetMathLibrary|NotEqualExactlyVectorVector _returnvalue "0, 0, 0")
    ;[1 1 1] Deals with the animation changes
    (Sprite|SetFlipbook (Variables|Default|GetBall_Flipbook) (Variables|Flipbooks|GetBall%20Rotation_Flipbook))
    ;[1 1 1] Deals with the Velocity since the node before this kills it.
    (Physics|SetPhysicsLinearVelocity (Variables|Default|GetBall_Flipbook) (Variables|Default|GetCurrent%20Velocity) false "None")
    (else
      (Sprite|SetFlipbook (Variables|Default|GetBall_Flipbook) (Variables|Flipbooks|GetBall%20Idle_Flipbook)))))