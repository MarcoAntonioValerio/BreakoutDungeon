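; BP_HeadohoesSound is an audio actor that plays the headphones' music from wherever the headphones are.
; On BeginPlay it assigns HeadphonesSound to its AudioComponent, starts playback immediately and stores the BP_Headphones actor found with GetActorOfClass.
; Each Tick it moves the AudioComponent to that actor's location, so the sound follows the headphones without being attached to them.
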(event EventBeginPlay
  ;[1 1 1] Uses whatever sound we have in the headphones.
  (Audio|Components|Audio|SetSound (Variables|Components|GetAudioComponent) (Variables|Default|GetHeadphonesSound))
  ;[1 1 1] Plays that sound as soon as we start to enter the range which in our case is as soon as we play.
  (Audio|Components|Audio|Play (Variables|Components|GetAudioComponent) 0.0)
  ;[1 1 1] Stores the connection to the Headphones actor.
  (bind _returnvalue (Actor|GetActorOfClass "/Game/Blueprints/BP_Headphones.BP_Headphones_C"))
  (Variables|Default|SetHeadphonesActorReference _returnvalue))

(event EventTick
  (params (DeltaSeconds :type Float%20%28single-precision%29))
  ;[1 1 1] The music location is the same as the Headphones.
  (Transformation|SetWorldLocation (Variables|Components|GetAudioComponent) (Transformation|GetActorLocation (Variables|Default|GetHeadphonesActorReference)) false false))

(fn ConstructionScript)