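; Spell component for the player, centred on a Ball Recall spell that pulls BP_Ball_2 back to the player's hands.
; It caches player and ball references, and checks every frame whether any mana remains.
; Recall either redirects the ball's velocity when mana allows, or moves it over time when inside recall range.
; Helper events track that range, position its collider and sprite, play recall flipbooks and sound, and deplete mana.
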(event Custom|Recall%20Sprite%20Deactivate
  (bind _playeractorreference (Variables|References|GetPlayerActorReference))
  ;[0.3882 1 0.5623] Recall Spell
  ;;[1 1 1] Turn off recall sprite visibility.
  ;;;[1 1 1] Makes the Recal Collision Sprite Invisible.
  (Rendering|SetVisibility (Variables|/Game/Blueprints/BP_Player.BP_Player_C|GetCollisionRangeSprite _playeractorreference) false false)
  ;;;[1 1 1] Resets the animations counter.
  (Variables|/Game/Blueprints/BP_Player.BP_Player_C|SetBallRecall_Counter _playeractorreference 0))

(event Custom|Inside%20Recall%20Range
  (params (Other%20Actor :type Object%20Object%20Reference))
  ;[0.3882 1 0.5623] Recall Spell
  ;;[1 1 1] Checks if ball is in Recall range.
  (Utilities|Casting|CastToBP_Ball_2 Other%20Actor)
  (Variables|/Game/Blueprints/BP_Player.BP_Player_C|SetIsBallinsideRecallRange (Variables|References|GetPlayerActorReference) true))

(event Custom|Leaving%20Recall%20Range
  (params (Other%20Actor :type Object%20Object%20Reference))
  ;[0.3882 1 0.5623] Recall Spell
  ;;[1 1 1] Checks if ball is leaving the Recall range.
  (Utilities|Casting|CastToBP_Ball_2 Other%20Actor)
  (Variables|/Game/Blueprints/BP_Player.BP_Player_C|SetIsBallinsideRecallRange (Variables|References|GetPlayerActorReference) false))

(event Custom|Depleats%20One%20Shot%20of%20Magic
  (bind _playeractorreference (Variables|References|GetPlayerActorReference))
  ;[0.3882 1 0.5623] Recall Spell
  ;;[1 1 1] Depleats one bar (divided bars still to implement) of Magic.
  (Variables|/Game/Blueprints/BP_Player.BP_Player_C|SetCurrent%20Magic%20Quantity _playeractorreference (- (Variables|/Game/Blueprints/BP_Player.BP_Player_C|GetCurrent%20Magic%20Quantity _playeractorreference) (Variables|/Game/Blueprints/BP_Player.BP_Player_C|GetDepleat%20One%20bar%20Of%20Magiv%20Value _playeractorreference))))

(event Custom|Recall%20Range%20Sprite%20Activate
  (bind _playeractorreference (Variables|References|GetPlayerActorReference))
  (bind _collisionrangesprite (Variables|/Game/Blueprints/BP_Player.BP_Player_C|GetCollisionRangeSprite _playeractorreference))
  ;[0.3882 1 0.5623] Recall Spell
  ;;[1 1 1] Activates the Recall Range Sprite
  ;;;[1 1 1] Turns the visibility of the sprite on.
  (Rendering|SetVisibility _collisionrangesprite true false)
  ;;;[1 1 1] Updates the location of the collider.
  (Transformation|SetWorldLocation _collisionrangesprite (- (Transformation|GetWorldLocation (Variables|/Game/Blueprints/BP_Player.BP_Player_C|GetPlayer_Animation _playeractorreference)) (Variables|/Game/Blueprints/BP_Player.BP_Player_C|GetCollisionSprite_Offsett _playeractorreference)) false false))

(event Custom|Ball%20Returning
  (bind _playeractorreference (Variables|References|GetPlayerActorReference))
  ;[0.3882 1 0.5623] Recall Spell
  ;;[1 1 1] Ball Returning Custom Event
  ;;;[1 1 1] Checks if the ball is in recalling range.
  (if (Variables|/Game/Blueprints/BP_Player.BP_Player_C|GetIsBallinsideRecallRange _playeractorreference)
    ;;;[1 1 1] Gets the mesh of the Ball.
    (bind _returnvalue (Actor|GetActorOfClass "/Game/Blueprints/BP_Ball_2.BP_Ball_2_C"))
    ;;;[1 1 1] Kills the Velocity.
    (Physics|SetPhysicsLinearVelocity (Variables|/Game/Blueprints/BP_Ball_2.BP_Ball_2_C|GetBall_Mesh _returnvalue) "0, 0, 0" false "None")
    ;;;[1 1 1] Turns the can stop ball boolean on.
    (Variables|/Game/Blueprints/BP_Player.BP_Player_C|SetCanStopBall _playeractorreference true)
    ;;;[1 1 1] Currently lerps to the position of the player. Might have to change to something more related to getting the location of the player and trying to alter the trajectory of the ball to try to get back to the player.
    (Components|MoveComponentTo (Variables|/Game/Blueprints/BP_Ball_2.BP_Ball_2_C|GetBall_Mesh _returnvalue) (+ (Transformation|GetWorldLocation (Variables|/Script/Engine.Actor|GetRootComponent _playeractorreference)) (Variables|/Game/Blueprints/BP_Player.BP_Player_C|GetHandPositionForBallCatch _playeractorreference)) "0, 0, 0" false false 0.3 true)
    ;;;[1 1 1] Turn the boolean off.
    (Variables|/Game/Blueprints/BP_Player.BP_Player_C|SetCanStopBall _playeractorreference false)))

(event Custom|Recall%20Range%20Collision%20Position
  (bind _playeractorreference (Variables|References|GetPlayerActorReference))
  ;[0.3882 1 0.5623] Recall Spell
  ;;[1 1 1] Updates position of the Recall Collider.
  ;;;[1 1 1] Updates the location of the collider.
  (Transformation|SetWorldLocation (Variables|/Game/Blueprints/BP_Player.BP_Player_C|GetRecall_CollisionSphere _playeractorreference) (Transformation|GetWorldLocation (Variables|/Game/Blueprints/BP_Player.BP_Player_C|GetPlayer_Animation _playeractorreference)) false false))

(event Custom|Ball%20Recall%20Animations%20and%20Sound
  (bind _playeractorreference (Variables|References|GetPlayerActorReference))
  (bind _player_animation (Variables|/Game/Blueprints/BP_Player.BP_Player_C|GetPlayer_Animation _playeractorreference))
  ;[0.3882 1 0.5623] Recall Spell
  ;;[1 1 1] Ball recall animations and sound
  ;;;[1 1 1] Checks how many times the animations have played
  (if (== (Variables|/Game/Blueprints/BP_Player.BP_Player_C|GetBallRecall_Counter _playeractorreference) 0)
    ;;;[1 1 1] Ball Recall sound.
    (Audio|PlaySound2D (Variables|/Game/Blueprints/BP_Player.BP_Player_C|GetBallRecall_Sound _playeractorreference) 1.0 1.0 0.0 0 0)
    ;;;[1 1 1] Ball recall movement flipbook.
    (Sprite|SetFlipbook _player_animation (Variables|/Game/Blueprints/BP_Player.BP_Player_C|GetBallRecall_Movement_Flipbook _playeractorreference))
    ;;;[1 1 1] Waits for the ball recall movement to finish.
    (Utilities|FlowControl|Delay (Class|PaperFlipbookComponent|GetFlipbookLength _player_animation)))
  ;;;[1 1 1] Ball Recall Idle flipbook.
  (Sprite|SetFlipbook (Variables|/Game/Blueprints/BP_Player.BP_Player_C|GetPlayer_Animation _playeractorreference) (Variables|/Game/Blueprints/BP_Player.BP_Player_C|GetBallRecall_Idle_Flipbook _playeractorreference))
  ;;;[1 1 1] Adds one to the counter
  (Math|Integer|IncrementInt (Variables|/Game/Blueprints/BP_Player.BP_Player_C|GetBallRecall_Counter _playeractorreference)))

(event Custom|Mana%20Quantity%20Check
  ;[1 0 0.7231] General mana quantity check that will work with all the spells.
  ;;[1 1 1] Check if I have enough Mana for the spells.
  (if (> (Variables|/Game/Blueprints/BP_Player.BP_Player_C|GetCurrent%20Magic%20Quantity (Variables|References|GetPlayerActorReference)) 0.0)
    ;;[1 1 1] These 2 bools will be used to determine if I can do spells or not.
    (Variables|ControlBools|SetCanIUseSpells? true)
    (else
      (Variables|ControlBools|SetCanIUseSpells? false))))

(event Custom|Recall%20the%20Ball%20if%20Mana%20is%20Available
  ;[1 1 1] Ball Recall new Event
  ;;[1 1 1] Checks if I can use spells.
  (if (Math|Boolean|Equal(Boolean) (Variables|ControlBools|GetCanIUseSpells?) true)
    ;;[1 1 1] Stops the ball.
    (Physics|SetPhysicsLinearVelocity (Variables|/Game/Blueprints/BP_Ball_2.BP_Ball_2_C|GetBall_Mesh (Variables|References|GetBall%20Actor%20Reference)) "0, 0, 0" false "None")
    ;;[1 1 1] Turns the can stop ball boolean on.
    (Variables|/Game/Blueprints/BP_Player.BP_Player_C|SetCanStopBall (Variables|References|GetPlayerActorReference) true)
    ;;[1 1 1] Sends the Ball toward the Hands of the Player.
    (Physics|SetPhysicsLinearVelocity (Variables|/Game/Blueprints/BP_Ball_2.BP_Ball_2_C|GetBall_Mesh (Variables|References|GetBall%20Actor%20Reference)) (Math|Vector|GetUnitDirection(Vector) (Transformation|GetActorLocation (Variables|References|GetBall%20Actor%20Reference)) (Variables|/Game/Blueprints/BP_Player.BP_Player_C|GetHandPositionForBallCatch (Variables|References|GetPlayerActorReference))) false "None")
    (Development|PrintString "Ball Recall has Fired")))

(event EventBeginPlay
  ;[1 1 1] Storing the player reference into a variable.
  (bind _returnvalue (Actor|GetActorOfClass "/Game/Blueprints/BP_Player.BP_Player_C"))
  (Variables|References|SetPlayerActorReference _returnvalue)
  ;[1 1 1] Storing the Ball reference into a variable.
  (bind _returnvalue_2 (Actor|GetActorOfClass "/Game/Blueprints/BP_Ball_2.BP_Ball_2_C"))
  (Variables|References|SetBall%20Actor%20Reference _returnvalue_2))

(event EventTick
  (params (DeltaSeconds :type Float%20%28single-precision%29))
  ;[1 1 1] Checks if I have enough Mana to do spells at every frame.
  (CallFunction|ManaQuantityCheck))