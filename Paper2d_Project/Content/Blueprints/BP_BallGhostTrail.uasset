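; BP_BallGhostTrail is a short-lived afterimage actor that leaves a fading ghost sprite at the ball's position.
; BeginPlay caches the BP_Ball reference, which the GhostTrail event uses to copy a random frame from the ball's flipbook, move to its location and tint the sprite translucent pink.
; The GhostDisappear timeline then drives the sprite's scale and color to shrink and fade it, destroying the actor on finish.
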(event Custom|Ghost%20Trail
  (bind _ball_actor_reference (Variables|Default|GetBall%20Actor_Reference))
  (bind _ball_flipbook (Variables|/Game/Blueprints/BP_Ball.BP_Ball_C|GetBall_Flipbook _ball_actor_reference))
  (Rendering|Components|Sprite|SetSprite (Variables|Default|GetGhost) (Class|PaperFlipbook|GetSpriteatFrame (Class|PaperFlipbookComponent|GetFlipbook _ball_flipbook) (Math|Random|RandomIntegerinRange 1 (- (Class|PaperFlipbookComponent|GetFlipbookLengthinFrames _ball_flipbook) 1))))
  (Transformation|SetActorLocation (Transformation|GetActorLocation (Variables|Default|GetBall%20Actor_Reference)) false false)
  (Sprite|SetSpriteColor (Variables|Default|GetGhost) "(R=0.958333,G=0.539063,B=0.756446,A=0.875000)")
  (bind (_direction _scale_down_vector _fade_color_away) (Timeline|Ghost%20disappear PlayFromStart)
    (:Update
      (Transformation|SetWorldScale3D (Variables|Default|GetGhost) _scale_down_vector)
      (Sprite|SetSpriteColor (Variables|Default|GetGhost) _fade_color_away))
    (:Finished
      (Actor|DestroyActor))))

(event EventBeginPlay
  (bind _returnvalue (Actor|GetActorOfClass "/Game/Blueprints/BP_Ball.BP_Ball_C"))
  (Variables|Default|SetBall%20Actor_Reference _returnvalue))

(event Collision|EventActorBeginOverlap
  (params (OtherActor :type Actor%20Object%20Reference)))

(event EventTick
  (params (DeltaSeconds :type Float%20%28single-precision%29)))

(fn ConstructionScript)