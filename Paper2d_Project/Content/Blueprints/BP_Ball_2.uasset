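; BP_Ball_2 is a physics ball that the player holds before launching it.
; Every Tick it finds BP_Player via GetActorOfClass and, until HasBallBeenLaunched is set, moves itself to PlayerAnimation's location plus a hand offset.
; LaunchBall zeroes linear velocity to solve a launch bug, then applies LaunchImpulseVector as a velocity-change impulse.
; Directional launch control is still pending, and VelocityAndAngle is an empty stub.
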(event Custom|LaunchBall
  ;[0.375 0.6159 1] Ball Launch        ➡️ ⚽
  ;;[1 1 1] Resets the linear velicity (to solve launch bug)
  (Physics|SetPhysicsLinearVelocity (Variables|Default|GetBall_Mesh) "0, 0, 0" false "None")
  ;;[1 1 1] Adds the launching impulse to the ball!
  (Physics|AddImpulse (Variables|Default|GetBall_Mesh) (Variables|Default|GetLaunchImpulseVector) "None" true))

(event Custom|VelocityAndAngle)

(event Custom|BallPositionBeforeLaunch
  ;[1 0.4989 0.6718] Hold Ball in "hands" before launch.                   ✋⚽🤚
  (bind _returnvalue (Actor|GetActorOfClass "/Game/Blueprints/BP_Player.BP_Player_C"))
  (if (not (Variables|/Game/Blueprints/BP_Player.BP_Player_C|GetHasBallBeenLaunched _returnvalue))
    ;;[1 1 1] Keeps the ball glued to the Player
    (Transformation|SetActorLocation (+ (Transformation|GetWorldLocation (Variables|/Game/Blueprints/BP_Player.BP_Player_C|GetPlayer_Animation _returnvalue)) (Variables|/Game/Blueprints/BP_Player.BP_Player_C|GetHandPositionForBallCatch _returnvalue)) false false)))

(event EventBeginPlay
  ;[0.3953 1 0.5746] Event Begin Play
)

(event EventTick
  (params (DeltaSeconds :type Float%20%28single-precision%29))
  ;[0.3385 0.1265 0.14] Event Tick
  (CallFunction|BallPositionBeforeLaunch))

(fn ConstructionScript)