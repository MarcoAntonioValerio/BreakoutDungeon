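; BP_Player is the 2D paddle-style player character, moved vertically by physics impulses, that catches, launches and swats BP_Ball_2.
; Input sets state flags driving flipbooks, dash, brace and up/down swings, with attack and catcher boxes toggled during swings.
; Ball contact either catches it while CanStopBall is set or stuns the player with tint, camera shake and headphone knock-off.
; The Recall spell delegates range checks and per-tick recalling to ACSpells.
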(event OnComponentBeginOverlap(Attack_CollisionBox)
  (params (OverlappedComponent :type Primitive%20Component%20Object%20Reference) (OtherActor :type Actor%20Object%20Reference) (OtherComp :type Primitive%20Component%20Object%20Reference) (OtherBodyIndex :type Integer) (bFromSweep :type Boolean) (SweepResult :type Hit%20Result%20Structure%20%28by%20ref%29))
  ;[0.9949 1 0.6783] Attack nodes.    [[[[ToFinish]]]
  ;;[1 1 1] Attack collision box overlap.            👊🏾👊🏾👊🏾
  ;;;[1 1 1] Checks if I am swinging at the ball.
  (Utilities|Casting|CastToBP_Ball_2 OtherActor)
  ;;;[1 1 1] Checks what direction I am attacking, true means I am attacking up, false down.
  (if (Math|Boolean|NotEqual(Boolean) (Variables|Booleans|GetAmIAttackingDown) true)
    ;;;[1 1 1] Attack Events
    (CallFunction|SwingUp)
    (else
      (CallFunction|SwingDown))))

(event OnComponentBeginOverlap(Recall_CollisionSphere)
  (params (OverlappedComponent :type Primitive%20Component%20Object%20Reference) (OtherActor :type Actor%20Object%20Reference) (OtherComp :type Primitive%20Component%20Object%20Reference) (OtherBodyIndex :type Integer) (bFromSweep :type Boolean) (SweepResult :type Hit%20Result%20Structure%20%28by%20ref%29))
  ;[1 1 1] Ball recall collision range triggers.
  (Default|InsideRecallRange (Variables|Default|GetAC_Spells) OtherActor))

(event OnComponentBeginOverlap(BallCatcher_CollisionBox)
  (params (OverlappedComponent :type Primitive%20Component%20Object%20Reference) (OtherActor :type Actor%20Object%20Reference) (OtherComp :type Primitive%20Component%20Object%20Reference) (OtherBodyIndex :type Integer) (bFromSweep :type Boolean) (SweepResult :type Hit%20Result%20Structure%20%28by%20ref%29))
  ;[0.9949 1 0.6783] Attack nodes.    [[[[ToFinish]]]
  ;;[1 1 1] Swing down Nodes
  ;;;[0.2199 0.5565 1] On overlap with the ball.                      👩🏾‍🦱💥⚽
  (Utilities|Casting|CastToBP_Ball_2 OtherActor)
  ;;;;[1 1 1] Checks if I am holding the ball.
  (if (not (Variables|Booleans|GetAmIHoldingTheBall))
    ;;;;[1 1 1] Checks if I can stop the ball.
    (if (Variables|Booleans|GetCanStopBall)
      (Variables|Booleans|SetAmIHoldingTheBall true)
      (Variables|Booleans|SetAmIBracing false)
      (Variables|Booleans|SetCanStopBall false)
      (else
        ;;;;[1 1 1] Sets the Stun bool to true
        (Variables|Default|SetIsPlayerStunned? true)
        ;;;;[1 1 1] Fires the colour effect.
        (CallFunction|HitColourEffect)
        ;;;;[1 1 1] Fires the screen shake.
        (CallFunction|HitCameraShake)
        ;;;;[1 1 1] Sound when getting hit by ball.
        (Audio|PlaySound2D (Variables|Sounds|GetHitByBall_Sound) 1.0 1.0 0.0 0 0)
        ;;;;[1 1 1] Plays the "Getting Hit" aimation if you are not bracing.
        (Sprite|SetFlipbook (Variables|Default|GetPlayer_Animation) (Variables|Flipbooks|GetGettingHit_%20Flipbook))
        (bind _returnvalue (Actor|GetActorOfClass "/Game/Blueprints/BP_Headphones.BP_Headphones_C"))
        ;;;;[1 1 1] Check if I have the headphones on my head.
        (if (Variables|/Game/Blueprints/BP_Headphones.BP_Headphones_C|GetHeadphonesOnHead? _returnvalue)
          ;;;;[1 1 1] Plays the lose the headphones event.
          (Default|CollisionDirection/Player<=Ball _returnvalue)
          (Default|HeadphonesWentFlying _returnvalue))
        ;;;;[1 1 1] Unstuns the player.
        (Utilities|FlowControl|Delay 1.5)
        (Variables|Default|SetIsPlayerStunned? false)))))

(event OnComponentEndOverlap(Recall_CollisionSphere)
  (params (OverlappedComponent :type Primitive%20Component%20Object%20Reference) (OtherActor :type Actor%20Object%20Reference) (OtherComp :type Primitive%20Component%20Object%20Reference) (OtherBodyIndex :type Integer))
  ;[1 1 1] Ball recall collision range triggers.
  (Default|LeavingRecallRange (Variables|Default|GetAC_Spells) OtherActor))

(event Custom|Swing%20Sword%20Down
  ;[0.9949 1 0.6783] Attack nodes.    [[[[ToFinish]]]
  ;;[1 1 1] Swing down Nodes
  ;;;[0.2746 0.5762 1] Ball nodes.    ⚽⚽⚽
  ;;;;[0.5501 1 0.466] Handles Animation and Sound of Downward Swing    👊🏾⬇️
  ;;;;;[1 1 1] Checks how many times I have swinged already.
  (if (== (Variables|Default|GetTimesISwinged) 1)
    ;;;;;[1 1 1] Plays the swing animation.
    (Sprite|SetFlipbook (Variables|Default|GetPlayer_Animation) (Variables|Flipbooks|GetAttackDown_Flipbook))
    ;;;;;[1 1 1] Plays the Swing Down sound.
    (Audio|PlaySound2D (Variables|Sounds|GetAttackDown_Sound) 1.0 1.0 0.0 0 0)
    ;;;;;[1 1 1] Waits for the flipbook to finish.
    (Utilities|FlowControl|Delay (Class|PaperFlipbookComponent|GetFlipbookLength (Variables|Default|GetPlayer_Animation)))
    ;;;;;[1 1 1] Resets stuff to original state.
    (Variables|Booleans|SetAmIAttacking false)
    (Variables|Booleans|SetAmIAttackingDown false)
    (Collision|SetCollisionEnabled (Variables|Default|GetBallCatcher_CollisionBox) "QueryAndPhysics")
    (Collision|SetCollisionEnabled (Variables|Default|GetAttack_CollisionBox) "NoCollision")))

(event Custom|SwingDown
  ;[0.9949 1 0.6783] Attack nodes.    [[[[ToFinish]]]
  ;;[1 1 1] Swing down Nodes
  ;;;[0.1042 1 1] Down Swing force on ball.    ⚽⬇️
  ;;;;[1 1 1] Gets the mesh of the Ball.
  (bind _returnvalue (Actor|GetActorOfClass "/Game/Blueprints/BP_Ball_2.BP_Ball_2_C"))
  (Physics|SetPhysicsLinearVelocity (Variables|/Game/Blueprints/BP_Ball_2.BP_Ball_2_C|GetBall_Mesh _returnvalue) (Math|Vector|MakeVector (Variables|/Game/Blueprints/BP_Ball_2.BP_Ball_2_C|GetBallVelocity _returnvalue) 0.0 (Math|Random|RandomFloatinRange -3e+02 -4e+02)) false "None"))

(event Custom|Swing%20Sword%20Up
  ;[0.9949 1 0.6783] Attack nodes.    [[[[ToFinish]]]
  ;;[1 1 1] Swing up Nodes
  ;;;[1 1 1] Handles Animation and Sound of Upward Swing    👊🏾⬆️
  ;;;;[1 1 1] Checks how many times I have swinged already.
  (if (== (Variables|Default|GetTimesISwinged) 1)
    ;;;;[1 1 1] Plays the swing animation.
    (Sprite|SetFlipbook (Variables|Default|GetPlayer_Animation) (Variables|Flipbooks|GetAttackUp_Flipbook))
    ;;;;[1 1 1] Plays the Swing Down sound.
    (Audio|PlaySound2D (Variables|Sounds|GetAttackUp_Sound) 1.0 1.0 0.0 0 0)
    ;;;;[1 1 1] Waits for the flipbook to finish.
    (Utilities|FlowControl|Delay (Class|PaperFlipbookComponent|GetFlipbookLength (Variables|Default|GetPlayer_Animation)))
    ;;;;[1 1 1] Resets stuff to original state.
    (Variables|Booleans|SetAmIAttacking false)
    (Variables|Booleans|SetAmIAttackingUp false)
    (Collision|SetCollisionEnabled (Variables|Default|GetBallCatcher_CollisionBox) "QueryAndPhysics")
    (Collision|SetCollisionEnabled (Variables|Default|GetAttack_CollisionBox) "NoCollision")))

(event Custom|Swing%20Up
  ;[0.9949 1 0.6783] Attack nodes.    [[[[ToFinish]]]
  ;;[1 1 1] Swing up Nodes
  ;;;[1 1 1] Down Swing force on ball.    ⚽⬇️
  ;;;;[1 1 1] Gets the mesh of the Ball.
  (bind _returnvalue (Actor|GetActorOfClass "/Game/Blueprints/BP_Ball_2.BP_Ball_2_C"))
  (Physics|SetPhysicsLinearVelocity (Variables|/Game/Blueprints/BP_Ball_2.BP_Ball_2_C|GetBall_Mesh _returnvalue) (Math|Vector|MakeVector (Variables|/Game/Blueprints/BP_Ball_2.BP_Ball_2_C|GetBallVelocity _returnvalue) 0.0 (Math|Random|RandomFloatinRange 3e+02 4e+02)) false "None"))

(event Custom|Hit%20Colour%20Effect
  ;[0 0.9475 1] Effects      💥
  ;;[1 1 1] Player's hit effects
  ;;;[1 1 1] Hit Colour Effect
  (bind _returnvalue (Rendering|Material|CreateDynamicMaterialInstance (Variables|Default|GetPlayer_Animation) 0 "/Game/Materials/mat_PlayerSpriteMaterial.mat_PlayerSpriteMaterial" "None" :!class /Script/Engine.PrimitiveComponent))
  (bind _hit (Timeline|Timeline_0 PlayFromStart)
    (:Update
      (Rendering|Material|SetVectorParameterValue _returnvalue "Tint" _hit :!class /Script/Engine.MaterialInstanceDynamic))
    (:Finished
      (Rendering|Material|SetVectorParameterValue _returnvalue "Tint" "(R=1.000000,G=1.000000,B=1.000000,A=0.000000)" :!class /Script/Engine.MaterialInstanceDynamic))))

(event Custom|Hit%20Camera%20Shake
  ;[0 0.9475 1] Effects      💥
  ;;[1 1 1] Player's hit effects
  ;;;[1 1 1] Hit Screen Shake
  (CameraShakes|StartCameraShake (Game|GetPlayerCameraManager 0) "/Game/Blueprints/ShakeTest.ShakeTest_C" 1.0 "CameraLocal" "0, 0, 0"))

(event Custom|Set%20Player%20as%20Listener
  ;[1 0.6254 0.09543] Sets the Player as the Music Listener.
  (Class|PlayerController|SetAudioListenerOverride (Game|GetPlayerController 0) (Variables|Default|GetPlayer_Animation) "0, 0, 0" "0, 0, 0"))

(event EventBeginPlay
  (bind _recall_collisionsphere (Variables|Default|GetRecall_CollisionSphere))
  ;[0.4439 1 0.2916] Begin Play
  ;;[1 1 1] Fires the Create UI event from the UIManager actor.
  (bind _returnvalue (Actor|GetActorOfClass "/Game/Blueprints/MAN_UiManager.MAN_UiManager_C"))
  (Default|CreateUI _returnvalue)
  (CallFunction|SetPlayerasListener)
  ;;[1 1 1] Disables the Attack collision on start.
  (Collision|SetCollisionEnabled (Variables|Default|GetAttack_CollisionBox) "NoCollision")
  ;;[1 1 1] Spell stuff.
  (Utilities|WhatSpellAmIUsing
    (:Recall
      ;;;[1 1 1] Enables the Recall Collision Sphere if we are using the Recall spell.
      (Collision|SetCollisionEnabled _recall_collisionsphere "QueryAndPhysics")
      ;;;[1 1 1] Stores the radius of the collider.
      (Variables|Default|SetCollision%20Sphere%20Radius (Components|Sphere|GetScaledSphereRadius _recall_collisionsphere))
      ;;;[1 1 1] Getting half of the sprite X.
      (Variables|Default|SetCollision%20Sprite%20Half%20X (/ (.x (Transformation|GetWorldScale (Variables|Default|GetCollisionRangeSprite))) 2.0)))
    (:Burst
      ;;;[1 1 1] Disables the Recall Collision Sphere if we are using the Burst spell.
      (Collision|SetCollisionEnabled (Variables|Default|GetRecall_CollisionSphere) "NoCollision"))))

(event EventTick
  (params (DeltaSeconds :type Float%20%28single-precision%29))
  (bind _ac_spells (Variables|Default|GetAC_Spells))
  ;[1 0.07339 0.2032] Event Tick
  ;;[1 1 1] Fires every frame.
  ;;[1 1 1] Checks what spell is active.
  (Utilities|WhatSpellAmIUsing
    (:Recall
      ;;[1 1 1] Recall Spell
      ;;;[1 1 1] Checks if I am recalling the Ball
      (if (Variables|Booleans|GetIAmPressingToRecallTheball)
        ;;;[1 1 1] Event called from the AC_Spells component.
        (Default|RecalltheBallifManaIsAvailable _ac_spells)
        (Default|BallRecallAnimationsandSound _ac_spells)))))

(event Input|ActionEvents|InputActionTesting
  (params (Key :type Key%20Structure :default "None"))
  ;[1 1 1] Inputs
)

(event Input|ActionEvents|InputActionSwingUp
  (params (Key :type Key%20Structure :default "None"))
  ;[1 1 1] Inputs
  ;;[1 1 1] Swing Up Input Trigger
  (:Pressed
    ;;;[1 1 1] Checks if I am holding the ball.
    (if (not (Variables|Booleans|GetAmIHoldingTheBall))
      ;;;[1 1 1] Deactivates the BallCatcher collision.
      (Collision|SetCollisionEnabled (Variables|Default|GetBallCatcher_CollisionBox) "NoCollision")
      ;;;[1 1 1] Activates the Attack collision.
      (Collision|SetCollisionEnabled (Variables|Default|GetAttack_CollisionBox) "QueryAndPhysics")
      ;;;[1 1 1] Checks if I am already attacking Up
      (if (Math|Boolean|NotEqual(Boolean) (Variables|Booleans|GetAmIAttackingDown) true)
        ;;;[1 1 1] Control variables.
        (Variables|Booleans|SetAmIAttacking true)
        (Variables|Booleans|SetAmIAttackingUp true)
        (Variables|Default|SetTimesISwinged 1))))
  (:Released
    ;;;[1 1 1] Resets the swing counter.
    (Variables|Default|SetTimesISwinged 0)))

(event Input|ActionEvents|InputActionDash/Brace
  (params (Key :type Key%20Structure :default "None"))
  ;[1 1 1] Inputs
  ;;[1 0.968 0.3904] Dashing /Bracing   👩🏾‍🦱💨💨
  (:Pressed
    ;;;[1 1 1] Checks if I am Attacking.
    (if (not (Variables|Booleans|GetAmIAttacking))
      ;;;[1 1 1] Check if we are moving, otherwise Brace.
      (if (!= (Math|Float|Truncate (Variables|Default|GetPaddle%20Direction)) 0)
        ;;;[1 1 1] The dashing recovery time is true
        (if (Variables|Default|GethaveiRecoverdFromDashing)
          ;;;[1 1 1] Set dashing recovery time to false
          (Variables|Default|SethaveiRecoverdFromDashing false)
          ;;;[1 1 1] Sets Dashing to True
          (Variables|Booleans|SetamIDashing true)
          (Variables|Booleans|SetCanStopBall true)
          ;;;[1 1 1] This is the Dash animation.
          (Sprite|SetFlipbook (Variables|Default|GetPlayer_Animation) (Variables|Flipbooks|GetDashRoll_Flipbook))
          ;;;[1 1 1] Check what direction the paddle is going
          (switch int (Math|Float|Truncate (Variables|Default|GetPaddle%20Direction))
            (:-1
              ;;;[1 1 1] Gives downward force to the Paddle
              (Physics|AddImpulse (Variables|Default|GetPlayer_Animation) (Math|Vector|MakeVector 0.0 0.0 (* -1.0 (Variables|Default|GetDashForce))) "None" true))
            (:1
              ;;;[1 1 1] Gives upward force to the Paddle
              (Physics|AddImpulse (Variables|Default|GetPlayer_Animation) (Math|Vector|MakeVector 0.0 0.0 (* 1.0 (Variables|Default|GetDashForce))) "None" true)))
          ;;;[1 1 1] Delay before being able to move after the dash.
          (Utilities|FlowControl|Delay (Class|PaperFlipbookComponent|GetFlipbookLength (Variables|Default|GetPlayer_Animation)))
          ;;;[1 1 1] Resetting Variables.
          (Variables|Booleans|SetamIDashing false)
          (Variables|Default|SethaveiRecoverdFromDashing true)
          (Variables|Booleans|SetAmIAttacking false)
          (Variables|Booleans|SetCanStopBall false))
        (else
          ;;;[1 1 1] Bracing nodes.
          ;;;;[1 1 1] Checks if I am holding the ball.
          (if (Variables|Booleans|GetAmIHoldingTheBall)
            (Variables|Booleans|SetAmIBracing false)
            (else
              (Variables|Booleans|SetAmIBracing true)
              (Variables|Booleans|SetCanStopBall true)
              ;;;;[1 1 1] How long will the brace last, duration will need to be the length of the Animation when finished.
              (Utilities|FlowControl|Delay (Variables|Default|GetBracingDuration))
              ;;;;[1 1 1] Resetting variables
              (Variables|Booleans|SetAmIBracing false)
              (Variables|Booleans|SetCanStopBall false))))))))

(event Input|ActionEvents|InputActionSpell
  (params (Key :type Key%20Structure :default "None"))
  ;[1 1 1] Inputs
  ;;[0.1729 0.9203 1] Spells Input
  (:Pressed
    ;;;[1 1 1] Check if I am holding the ball.
    (if (not (Variables|Booleans|GetAmIHoldingTheBall))
      (Variables|Booleans|SetIAmPressingSpellButton true)
      ;;;[1 1 1] Check what spell is active.
      (Utilities|WhatSpellAmIUsing
        (:Recall
          ;;;[1 1 1] Recall
          ;;;;[1 1 1] Checks the counter, and do not fire if it has already ran once.
          (if (== (Variables|SpellsStuff|GetSpell%20Firing%20Counter) 0)
            ;;;;[1 1 1] Turns on recall boolean.
            (Variables|Booleans|SetIAmPressingToRecallTheball true)
            ;;;;[1 1 1] Adds one to the counter
            (Math|Integer|IncrementInt (Variables|SpellsStuff|GetSpell%20Firing%20Counter)
              (:%20%20
                ;;;;[1 1 1] Fires the Depleat Magic event.
                (Development|PrintString "Spell Pressed"))))))))
  (:Released
    (Variables|Booleans|SetIAmPressingSpellButton false)
    ;;;[1 1 1] Check what spell is active.
    (Utilities|WhatSpellAmIUsing
      (:Recall
        ;;;[1 1 1] Recall
        ;;;;[1 1 1] Turns off recall boolean.
        (Variables|Booleans|SetIAmPressingToRecallTheball false)
        ;;;;[1 1 1] Resets the counter.
        (Variables|SpellsStuff|SetSpell%20Firing%20Counter 0)
        (Variables|Booleans|SetCanStopBall false)))))

(event Input|ActionEvents|InputActionSwingDown
  (params (Key :type Key%20Structure :default "None"))
  ;[1 1 1] Inputs
  ;;[1 1 1] Swing Down Input Trigger
  (:Pressed
    ;;;[1 1 1] Checks if I am holding the ball.
    (if (not (Variables|Booleans|GetAmIHoldingTheBall))
      ;;;[1 1 1] Deactivates the BallCatcher collision.
      (Collision|SetCollisionEnabled (Variables|Default|GetBallCatcher_CollisionBox) "NoCollision")
      ;;;[1 1 1] Activates the Attack collision.
      (Collision|SetCollisionEnabled (Variables|Default|GetAttack_CollisionBox) "QueryAndPhysics")
      ;;;[1 1 1] Checks if I am already attacking Up
      (if (Math|Boolean|NotEqual(Boolean) (Variables|Booleans|GetAmIAttackingUp) true)
        ;;;[1 1 1] Control variables.
        (Variables|Booleans|SetAmIAttacking true)
        (Variables|Booleans|SetAmIAttackingDown true)
        (Variables|Default|SetTimesISwinged 1))))
  (:Released
    ;;;[1 1 1] Resets the swing counter.
    (Variables|Default|SetTimesISwinged 0)
    ;;;[1 1 1] Turn off the IAmPressingTheSpellButton boolean
    (Variables|Booleans|SetIAmPressingSpellButton false)))

(event Input|ActionEvents|InputActionShootBall
  (params (Key :type Key%20Structure :default "None"))
  ;[0.9949 1 0.6783] Attack nodes.    [[[[ToFinish]]]
  ;;[1 1 1] Swing down Nodes
  ;;;[0.2746 0.5762 1] Ball nodes.    ⚽⚽⚽
  ;;;;[1 1 1] Ball launch button.         👊🏾⚽   [[[[[[[[[[[[[TOFINISH]]]]]]]]]]]]
  (:Pressed
    ;;;;;[1 1 1] Checks if the Ball the player is holding the ball.
    (if (Variables|Booleans|GetAmIHoldingTheBall)
      ;;;;;[1 1 1] Sets the bool to true.
      (Variables|Booleans|SetAmILaunchingTheBall true)
      ;;;;;[1 1 1] Does the launch animation
      (Sprite|SetFlipbook (Variables|Default|GetPlayer_Animation) (Variables|Flipbooks|GetLaunchBall_Flipbook))
      ;;;;;[1 1 1] Ball launch sound.
      (Audio|PlaySound2D (Variables|Sounds|GetBallLaunch_Sound) 1.0 1.0 0.0 0 0)
      ;;;;;[1 1 1] Creates a delay to wait for the launch animation to be finished.
      (Utilities|FlowControl|Delay (Class|PaperFlipbookComponent|GetFlipbookLength (Variables|Default|GetPlayer_Animation)))
      ;;;;;[1 1 1] Fires the launch Ball event from the BP_Ball2 actor.
      (bind _returnvalue (Actor|GetActorOfClass "/Game/Blueprints/BP_Ball_2.BP_Ball_2_C"))
      (Default|LaunchBall _returnvalue)
      ;;;;;[1 1 1] Sets both booleans to false since I have launcged the ball.
      (Variables|Booleans|SetAmIHoldingTheBall false)
      (Variables|Booleans|SetAmILaunchingTheBall false))))

(event Input|AxisEvents|InputAxisVerticalMovement
  (params (AxisValue :type Float%20%28single-precision%29))
  ;[1 1 1] Inputs
  ;;[0.5836 0.4491 1] Deals with Vertical movement.      ↕️👩🏾‍🦱
  ;;;[1 1 1] This will give me the axis direction
  (Variables|Default|SetPaddle%20Direction AxisValue)
  ;;;[1 1 1] Checks if the player is stunned.
  (if (Variables|Default|GetIsPlayerStunned?)
    ;;;[1 1 1] Stunned animation.
    (Sprite|SetFlipbook (Variables|Default|GetPlayer_Animation) (Variables|Flipbooks|GetStunned_Flipbook))
    (else
      ;;;[1 1 1] Checks if I am bracing.
      (if (Variables|Booleans|GetAmIBracing)
        ;;;[1 1 1] Swaps to the bracing animation.
        (Sprite|SetFlipbook (Variables|Default|GetPlayer_Animation) (Variables|Flipbooks|GetBracing_Flipbook))
        (else
          ;;;[1 1 1] Checks if we are dashing
          (if (not (Variables|Booleans|GetamIDashing))
            ;;;[1 1 1] Checks if I am launching the ball.
            (if (not (Variables|Booleans|GetAmILaunchingTheBall))
              ;;;[1 1 1] Checks if I am moving.
              (if (!= AxisValue 0.0)
                ;;;[1 1 1] Checks if I am attacking.
                (if (Math|Boolean|Equal(Boolean) (Variables|Booleans|GetAmIAttacking) true)
                  ;;;[1 1 1] Checks if I am attacking up, if FALSE i am attacking down.
                  (if (Math|Boolean|Equal(Boolean) (Variables|Booleans|GetAmIAttackingUp) true) :!label _label
                    ;;;[1 1 1] Fires the event.
                    (CallFunction|SwingSwordUp)
                    (else
                      (CallFunction|SwingSwordDown)))
                  (else
                    ;;;[1 1 1] Sets the flipbooks for the animations.
                    (Sprite|SetFlipbook (Variables|Default|GetPlayer_Animation) (Variables|Flipbooks|GetMove_Flipbook))
                    ;;;[1 1 1] Gives force to the Paddle
                    (Physics|AddImpulse (Variables|Default|GetPlayer_Animation) (Math|Vector|MakeVector 0.0 0.0 (* (* (Variables|Default|GetSpeed) AxisValue (Utilities|Time|GetWorldDeltaSeconds)) 1e+02)) "None" false :!label _label_2)))
                (else
                  ;;;[1 1 1] Checks if I am attacking.
                  (if (Math|Boolean|Equal(Boolean) (Variables|Booleans|GetAmIAttacking) true)
                    (goto _label)
                    (else
                      (Sprite|SetFlipbook (Variables|Default|GetPlayer_Animation) (Variables|Flipbooks|GetIdle_Flipbook))
                      (goto _label_2))))))))))))

(fn ConstructionScript)