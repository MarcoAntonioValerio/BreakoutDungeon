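; Paper2D headphones actor that the player wears, can lose and can pick back up.
; While worn, Tick looks up BP_Player each frame, snaps the flipbook to its head pivot plus an offset, sets the on-head animation and disables collision.
; HeadphonesWentFlying fakes three bounces with directional, then shrinking upward impulses, delays and gravity toggles.
; Pickup unlocks after the last bounce, so overlapping the player puts them back on.
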(event OnComponentBeginOverlap(Headphones_Flipbook)
  (params (OverlappedComponent :type Primitive%20Component%20Object%20Reference) (OtherActor :type Actor%20Object%20Reference) (OtherComp :type Primitive%20Component%20Object%20Reference) (OtherBodyIndex :type Integer) (bFromSweep :type Boolean) (SweepResult :type Hit%20Result%20Structure%20%28by%20ref%29))
  ;[1 1 1] If the player overlaps with the fallen headphones.
  ;;[1 1 1] Checks if I am overlapping with the player.
  (Utilities|Casting|CastToBP_Player OtherActor)
  ;;[1 1 1] Check if the headphones are still flying away.
  (if (Variables|Default|GetCanIPickHeadphonesUp?)
    (Variables|Default|SetHeadphonesOnHead? true)))

(event Custom|Headphones%20are%20on%20Head
  ;[1 1 1] Headphones on Head Event
  ;;[1 1 1] Gets the player
  (bind _returnvalue (Actor|GetActorOfClass "/Game/Blueprints/BP_Player.BP_Player_C"))
  ;;[1 1 1] Moves this actor (thus the Headphones) to the pivot I have set on the player.
  (Transformation|SetWorldLocation (Variables|Default|GetHeadphones_Flipbook) (+ (Transformation|GetWorldLocation (Variables|/Game/Blueprints/BP_Player.BP_Player_C|GetHeadPhones_Location _returnvalue)) (Variables|Default|GetHeadphones%20Offset)) false false)
  ;;[1 1 1] Changes the flipbook to the one where the headphones are on the head.
  (Sprite|SetFlipbook (Variables|Default|GetHeadphones_Flipbook) "/Game/Assets/test_Characters/anim_headphonesOnHead.anim_HeadphonesOnHead")
  ;;[1 1 1] Deactivates the headphones collision.
  (Collision|SetCollisionEnabled (Variables|Default|GetHeadphones_Flipbook) "NoCollision"))

(event Custom|Headphones%20Went%20Flying
  ;[1 1 1] Event to lose headphones
  ;;[1 1 1] Deactivates booleans.
  (Variables|Default|SetCanIPickHeadphonesUp? false)
  (Variables|Default|SetHeadphonesOnHead? false)
  ;;[1 1 1] Reacttivates the Collision physics.
  (Collision|SetCollisionEnabled (Variables|Default|GetHeadphones_Flipbook) "QueryAndPhysics")
  ;;[1 1 1] First Bounce
  (Physics|AddImpulse (Variables|Default|GetHeadphones_Flipbook) (Utilities|Select :Index (Variables|Default|GetEjection%20Direction) :NewEnumerator0 (Variables|Default|GetUpward_ImpulseToHeadphones) :NewEnumerator1 (Variables|Default|GetDownward_ImpulseToHeadphones)) "None" true)
  (Physics|SetEnableGravity (Variables|Default|GetHeadphones_Flipbook) (Utilities|Enum|Equal(Enum) (Variables|Default|GetEjection%20Direction) "NewEnumerator0"))
  (Utilities|FlowControl|Delay 0.5)
  (Class|PrimitiveComponent|SetAllPhysicsLinearVelocity (Variables|Default|GetHeadphones_Flipbook) "0, 0, 0" false)
  (Physics|SetEnableGravity (Variables|Default|GetHeadphones_Flipbook) false)
  ;;[1 1 1] Second Bounce
  (Physics|AddImpulse (Variables|Default|GetHeadphones_Flipbook) (/ (Variables|Default|GetUpward_ImpulseToHeadphones) 2.0) "None" true)
  (Physics|SetEnableGravity (Variables|Default|GetHeadphones_Flipbook) true)
  (Utilities|FlowControl|Delay 0.5)
  (Class|PrimitiveComponent|SetAllPhysicsLinearVelocity (Variables|Default|GetHeadphones_Flipbook) "0, 0, 0" false)
  (Physics|SetEnableGravity (Variables|Default|GetHeadphones_Flipbook) false)
  ;;[1 1 1] Third Bounce
  (Physics|AddImpulse (Variables|Default|GetHeadphones_Flipbook) (/ (Variables|Default|GetUpward_ImpulseToHeadphones) 4.0) "None" true)
  (Physics|SetEnableGravity (Variables|Default|GetHeadphones_Flipbook) true)
  (Utilities|FlowControl|Delay 0.25)
  (Class|PrimitiveComponent|SetAllPhysicsLinearVelocity (Variables|Default|GetHeadphones_Flipbook) "0, 0, 0" false)
  (Physics|SetEnableGravity (Variables|Default|GetHeadphones_Flipbook) false)
  ;;[1 1 1] Makes headphones pickapable.
  (Variables|Default|SetCanIPickHeadphonesUp? true))

(event EventBeginPlay)

(event Collision|EventActorBeginOverlap
  (params (OtherActor :type Actor%20Object%20Reference)))

(event EventTick
  (params (DeltaSeconds :type Float%20%28single-precision%29))
  ;[1 1 1] Checks if the "Headphones on Head!" variable is true.
  (if (Variables|Default|GetHeadphonesOnHead?)
    (CallFunction|HeadphonesAreonHead)))

(fn ConstructionScript)